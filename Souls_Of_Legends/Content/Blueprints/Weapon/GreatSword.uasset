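; Great sword weapon actor that damages the player's current boss, a Fiddlesticks_BP, on hitbox overlap.
; BeginPlay caches the player character and disables the hitbox, which ToggleHitbox switches on or off.
; While CanHit is true, an overlap deals higher damage during a sprint attack and then clears CanHit.
; Normal hits deal base damage and leave CanHit set.
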(event OnComponentBeginOverlap(hitbox)
  (params (OverlappedComponent :type Primitive%20Component%20Object%20Reference) (OtherActor :type Actor%20Object%20Reference) (OtherComp :type Primitive%20Component%20Object%20Reference) (OtherBodyIndex :type Integer) (bFromSweep :type Boolean) (SweepResult :type Hit%20Result%20Structure%20%28by%20ref%29))
  (if (Variables|Default|Getcan_hit)
    (if (== OtherActor (Variables|/Game/ThirdPersonBP/Blueprints/ThirdPersonCharacter.ThirdPersonCharacter_C|Getcurrent_boss (Variables|Default|Getplayer)))
      (bind _asfiddlesticks_bp (Utilities|Casting|CastToFiddlesticks_BP (Variables|/Game/ThirdPersonBP/Blueprints/ThirdPersonCharacter.ThirdPersonCharacter_C|Getcurrent_boss (Variables|Default|Getplayer))))
      (if (Variables|/Game/ThirdPersonBP/Blueprints/ThirdPersonCharacter.ThirdPersonCharacter_C|Getsprint_attack (Variables|Default|Getplayer))
        (Default|TakeDamage _asfiddlesticks_bp 2e+02)
        (Variables|Default|Setcan_hit false)
        (else
          (Default|TakeDamage _asfiddlesticks_bp 1e+02))))))

(event EventBeginPlay
  (bind _asthird_person_character (Utilities|Casting|CastToThirdPersonCharacter (Game|GetPlayerCharacter 0)))
  (Variables|Default|Setplayer _asthird_person_character)
  (Collision|SetCollisionEnabled (Variables|Default|Gethitbox) "NoCollision"))

(event Collision|EventActorBeginOverlap
  (params (OtherActor :type Actor%20Object%20Reference)))

(event EventTick
  (params (DeltaSeconds :type Float%20%28single-precision%29)))

(fn ConstructionScript)

(fn ToggleHitbox
  (params (toggle :type Boolean))
  (bind _hitbox (Variables|Default|Gethitbox))
  (if toggle
    (Collision|SetCollisionEnabled _hitbox "QueryAndPhysics")
    (else
      (Collision|SetCollisionEnabled _hitbox "NoCollision"))))