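; Fog door actor that can be triggered to show its particle effect and enable a blocker, apparently for boss encounters.
; The blocker starts without collision; overlapping the interact box registers the door on the player.
; TriggerGate activates the fog and query-only blocker collision, while ToggleCollision sets blocking or ignore responses.
; AddBossUi creates the boss HP widget, but its call in ToggleCollision is disconnected, as is the hint-hiding logic.
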(event OnComponentBeginOverlap(interact_box)
  (params (OverlappedComponent :type Primitive%20Component%20Object%20Reference) (OtherActor :type Actor%20Object%20Reference) (OtherComp :type Primitive%20Component%20Object%20Reference) (OtherBodyIndex :type Integer) (bFromSweep :type Boolean) (SweepResult :type Hit%20Result%20Structure%20%28by%20ref%29))
  (Variables|/Game/ThirdPersonBP/Blueprints/ThirdPersonCharacter.ThirdPersonCharacter_C|Settouched_fog_door (Variables|Default|Getplayer) self))

(event OnComponentEndOverlap(interact_box)
  (params (OverlappedComponent :type Primitive%20Component%20Object%20Reference) (OtherActor :type Actor%20Object%20Reference) (OtherComp :type Primitive%20Component%20Object%20Reference) (OtherBodyIndex :type Integer)))

(event EventBeginPlay
  (bind _asthird_person_character (Utilities|Casting|CastToThirdPersonCharacter (Game|GetPlayerCharacter 0)))
  (Variables|Default|Setplayer _asthird_person_character)
  (Collision|SetCollisionEnabled (Variables|Default|Getblocker) "NoCollision"))

(event Collision|EventActorBeginOverlap
  (params (OtherActor :type Actor%20Object%20Reference)))

(event EventTick
  (params (DeltaSeconds :type Float%20%28single-precision%29)))

(fn ConstructionScript)

(fn ToggleCollision
  (params (toggle :type Boolean))
  (if toggle
    (Collision|SetCollisionResponsetoAllChannels (Variables|Default|Getblocker) "ECR_Block")
    (else
      (Collision|SetCollisionResponsetoAllChannels (Variables|Default|Getblocker) "ECR_Ignore")
      (Collision|SetCollisionResponsetoAllChannels (Variables|Default|Getinteract_box) "ECR_Ignore"))))

(fn AddBossUi
  (bind _returnvalue (UserInterface|CreateWidget "/Game/Widgets/Boss_HP.Boss_HP_C" 0 0))
  (UserInterface|Viewport|AddtoViewport _returnvalue 0))

(fn TriggerGate
  (Components|Activation|Activate (Variables|Default|GetParticleSystem) false)
  (Collision|SetCollisionEnabled (Variables|Default|Getblocker) "QueryOnly"))