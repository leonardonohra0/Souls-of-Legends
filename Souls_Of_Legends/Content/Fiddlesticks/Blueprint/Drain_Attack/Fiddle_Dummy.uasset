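; Fiddle_Dummy is an actor that hosts a Drain_Attack actor between itself and the player, in the Fiddlesticks content.
; On BeginPlay it caches the ThirdPersonCharacter, then spawns a Drain_Attack at the midpoint between its Cylinder and the player and attaches it to itself.
; Each Tick it rotates to face the player and moves the attached attack back to that midpoint.
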(event EventBeginPlay
  (bind _asthird_person_character (Utilities|Casting|CastToThirdPersonCharacter (Game|GetPlayerCharacter 0)))
  (Variables|Default|Setplayer _asthird_person_character)
  (bind _returnvalue (Game|SpawnActorfromClass "/Game/Fiddlesticks/Blueprint/Drain_Attack/Drain_Attack.Drain_Attack_C" (Math|Transform|MakeTransform (/ (+ (Transformation|GetWorldLocation (Variables|Default|GetCylinder)) (Transformation|GetActorLocation (Variables|Default|Getplayer))) 2.0) "0, 0, 0" "1,1,1") "Undefined" 0 0))
  (Transformation|AttachActorToActor _returnvalue self "None" "SnapToTarget" "SnapToTarget" "SnapToTarget" true))

(event Collision|EventActorBeginOverlap
  (params (OtherActor :type Actor%20Object%20Reference)))

(event EventTick
  (params (DeltaSeconds :type Float%20%28single-precision%29))
  (Transformation|SetActorRotation (Math|Rotator|FindLookatRotation (Transformation|GetActorLocation) (Transformation|GetActorLocation (Variables|Default|Getplayer))))
  (Transformation|SetActorLocation (stale EventBeginPlay _returnvalue) (/ (+ (Transformation|GetWorldLocation (Variables|Default|GetCylinder)) (Transformation|GetActorLocation (Variables|Default|Getplayer))) 2.0) false false))

(fn ConstructionScript)