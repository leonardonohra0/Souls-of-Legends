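; Fiddlesticks enemy character that screeches when the player first comes within range, then chases and slashes at close range.
; BeginPlay caches the ThirdPersonCharacter and attaches a spawned effect actor to the scythe socket.
; GetPlayerDistance switches movement and montages by distance, using FirstTime and CanAttack flags.
; Helper functions handle damage and death state, grow the drain effect, and toggle a lock-on dot on the spine.
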(event Custom|death_event
  (Utilities|FlowControl|Delay 5.0))

(event EventBeginPlay
  (bind _asthird_person_character (Utilities|Casting|CastToThirdPersonCharacter (Game|GetPlayerCharacter 0)))
  (Variables|Default|Setplayer _asthird_person_character)
  (bind _returnvalue (Game|SpawnActorfromClass "/Game/Fiddlesticks/Blueprint/Slash_Attack/PS_reference.PS_reference_C" (Transformation|GetSocketTransform (Variables|Character|GetMesh) "scythe_PS" "RTS_World") "Undefined" 0 0))
  (bind _output_get (Variables|Default|Setps_ref _returnvalue))
  (Transformation|AttachComponentToComponent _output_get (Variables|Character|GetMesh) "scythe_PS" "SnapToTarget" "SnapToTarget" "SnapToTarget" false))

(event Collision|EventActorBeginOverlap
  (params (OtherActor :type Actor%20Object%20Reference)))

(event EventTick
  (params (DeltaSeconds :type Float%20%28single-precision%29)))

(fn ConstructionScript)

(fn GetPlayerDistance
  (if (Variables|Default|Getfirst_time)
    (if (< (Math|Vector|Distance(Vector) (Transformation|GetWorldLocation (Variables|/Script/Engine.Character|GetMesh (Variables|Default|Getplayer))) (Transformation|GetWorldLocation (Variables|Character|GetMesh))) 3.5e+03)
      (Variables|Default|Setfirst_time false)
      (Animation|PlayAnimMontage "/Game/Fiddlesticks/Animations/Montages/Fiddle_screech.Fiddle_screech" 1.0 "None"))
    (elif (< (Math|Vector|Distance(Vector) (Transformation|GetWorldLocation (Variables|/Script/Engine.Character|GetMesh (Variables|Default|Getplayer))) (Transformation|GetWorldLocation (Variables|Character|GetMesh))) 1e+03)
      (Pawn|Components|CharacterMovement|SetMovementMode (Variables|Character|GetCharacterMovement) "MOVE_None" 0)
      (Variables|Default|Setshould_move false)
      (if (Variables|Default|Getcan_attack)
        (Variables|Default|Setcan_attack false)
        (Animation|PlayAnimMontage "/Game/Fiddlesticks/Animations/Montages/wide_slash_attack.wide_slash_attack" 0.75 "None"))
      (elif (not (Variables|Default|Getcan_attack))
        (Variables|Default|Setshould_move true)
        (Pawn|Components|CharacterMovement|SetMovementMode (Variables|Character|GetCharacterMovement) "MOVE_Walking" 0)
        (AI|Navigation|SimpleMovetoActor (Pawn|GetController) (Variables|Default|Getplayer))))))

(fn TakeDamage
  (params (amount :type Float%20%28single-precision%29))
  (bind _output_get (Variables|Default|Sethealth (- (Variables|Default|Gethealth) amount)))
  (Variables|Default|Setis_dead (<= _output_get 0.0)))

(fn IncreaseChargeSize
  (bind _drain_ps (Variables|Default|Getdrain_PS))
  (Transformation|SetWorldScale3D _drain_ps (+ (Transformation|GetWorldScale _drain_ps) 0.1)))

(fn ToggleLockon
  (params (toggle :type Boolean))
  (bind _lockon_ref (Variables|Default|Getlockon_ref))
  (bind _returnvalue (Transformation|GetWorldTransform _lockon_ref))
  (if toggle
    (bind _returnvalue_2 (Game|SpawnActorfromClass "/Game/Fiddlesticks/Blueprint/lockon-dot.lockon-dot_C" (Math|Transform|MakeTransform (.location _returnvalue) (.rotation _returnvalue) "1,1,1") "Undefined" 0 0))
    (bind _output_get (Variables|Default|Setlock-on-actor _returnvalue_2))
    (Transformation|AttachComponentToComponent _output_get (Variables|Character|GetMesh) "Spine2" "SnapToTarget" "SnapToTarget" "SnapToTarget" true)
    (else
      (Actor|DestroyActor (Variables|Default|Getlock-on-actor)))))