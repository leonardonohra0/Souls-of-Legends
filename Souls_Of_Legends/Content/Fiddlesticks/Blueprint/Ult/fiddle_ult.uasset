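; Actor for Fiddlesticks' ultimate: a spinning black circle that damages the player standing inside it.
; BeginPlay caches the player as a ThirdPersonCharacter, and the circle's begin and end overlap events toggle a PlayerInside flag for that player only.
; Tick yaws the circle and applies damage every frame while the flag is set, so both spin and damage rate depend on frame rate.
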(event OnComponentBeginOverlap(circle_black)
  (params (OverlappedComponent :type Primitive%20Component%20Object%20Reference) (OtherActor :type Actor%20Object%20Reference) (OtherComp :type Primitive%20Component%20Object%20Reference) (OtherBodyIndex :type Integer) (bFromSweep :type Boolean) (SweepResult :type Hit%20Result%20Structure%20%28by%20ref%29))
  (if (== OtherActor (Game|GetPlayerCharacter 0))
    (Development|PrintString "Hello")
    (Variables|Default|Setplayer_inside true)))

(event OnComponentEndOverlap(circle_black)
  (params (OverlappedComponent :type Primitive%20Component%20Object%20Reference) (OtherActor :type Actor%20Object%20Reference) (OtherComp :type Primitive%20Component%20Object%20Reference) (OtherBodyIndex :type Integer))
  (if (== OtherActor (Game|GetPlayerCharacter 0))
    (Development|PrintString "Hello")
    (Variables|Default|Setplayer_inside false)))

(event EventBeginPlay
  (bind _asthird_person_character (Utilities|Casting|CastToThirdPersonCharacter (Game|GetPlayerCharacter 0)))
  (Variables|Default|Setplayer _asthird_person_character))

(event Collision|EventActorBeginOverlap
  (params (OtherActor :type Actor%20Object%20Reference)))

(event EventTick
  (params (DeltaSeconds :type Float%20%28single-precision%29))
  (bind _circle_black (Variables|Default|Getcircle_black))
  (bind _returnvalue (Transformation|GetWorldRotation _circle_black))
  (Transformation|SetWorldRotation _circle_black (Math|Rotator|MakeRotator (.roll _returnvalue) (.pitch _returnvalue) (+ (.yaw _returnvalue) 1.5)) false false)
  (if (Variables|Default|Getplayer_inside)
    (Default|TakeDamage (Variables|Default|Getplayer) 5.0)))

(fn ConstructionScript)